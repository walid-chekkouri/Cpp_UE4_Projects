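; Player pawn Pacman_BP with forward/back movement, a turning body and controller-driven camera look.
; RightLeft input yaws Body up to about 90 degrees either way; on release, a DoOnce reverses the step to rebound it to near zero.
; Movement uses swept, frame-rate-dependent SetActorLocation along control rotation, and TestMove pushes Body upward with force.
; Tick records FPS, while alternative rotation and movement methods remain disconnected.
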(event Custom|Resetter
  ;[0 0.3724 1] Smooth Rotation with a Smooth Snap back "AddRotationMethod"
  ;;[0.1416 1 0] Rebound
  (Utilities|FlowControl|DoOnce false) ; enters at Reset
)

(event EventTick
  (params (DeltaSeconds :type Float%20%28single-precision%29))
  ;[0 0.3724 1] Frames Per Second
  (Variables|Default|SetFPS (/ 1.0 DeltaSeconds)))

(event Input|AxisEvents|InputAxisTestMove
  (params (AxisValue :type Float%20%28single-precision%29))
  (Class|PrimitiveComponent|AddForceatLocation (Variables|Default|GetBody) "0, 0,300.000000" (Transformation|GetActorLocation) "None"))

(event Input|AxisEvents|InputAxisRightLeft
  (params (AxisValue :type Float%20%28single-precision%29))
  ;[0 0.3724 1] Smooth Rotation with a Smooth Snap back "AddRotationMethod"
  (if (== AxisValue 0.0)
    (Utilities|FlowControl|Sequence
      (:then_0
        ;;[0.1416 1 0] Rebound
        (Utilities|FlowControl|DoOnce false
          (:Completed
            (Variables|Default|SetToAdd (* (Variables|Default|GetToAdd) (* -1.0 (Utilities|Time|GetWorldDeltaSeconds)) (Variables|Default|GetReboundSpeed))))))
      (:then_1
        ;;[0.7812 0.01213 0] Limit Conditions
        (if (not (Math|Float|NearlyEqual(Float) (.yaw (Variables|/Script/Engine.SceneComponent|GetRelativeRotation (Variables|Default|GetBody))) 0.0 2.0))
          (Transformation|AddRelativeRotation (Variables|Default|GetBody) (Math|Rotator|MakeRotator 0.0 0.0 (Variables|Default|GetToAdd)) false false :!label _label))))
    (elif (> AxisValue 0.0)
      (Variables|Default|SetToAdd (* 8e+01 (Utilities|Time|GetWorldDeltaSeconds)))
      (if (not (>= (.yaw (Variables|/Script/Engine.SceneComponent|GetRelativeRotation (Variables|Default|GetBody))) 9e+01))
        (CallFunction|Resetter :!label _label_2)
        (goto _label))
      (elif (< AxisValue 0.0)
        (Variables|Default|SetToAdd (* -8e+01 (Utilities|Time|GetWorldDeltaSeconds)))
        (if (not (<= (.yaw (Variables|/Script/Engine.SceneComponent|GetRelativeRotation (Variables|Default|GetBody))) -9e+01))
          (goto _label_2))))))

(event Input|AxisEvents|InputAxisForwardBackward
  (params (AxisValue :type Float%20%28single-precision%29))
  ;[0 0.3724 1] Simple Forward Movement_Using "SetActorLocation" PS: Frame Rate Dependent Method
  (Transformation|SetActorLocation (+ (Transformation|GetActorLocation) (* (Math|Vector|GetForwardVector (Pawn|GetControlRotation :!class /Script/Engine.Pawn)) (* AxisValue (Math|Float|MakeLiteralFloat 4.0)))) true false))

(event Input|AxisEvents|InputAxisTurnRate
  (params (AxisValue :type Float%20%28single-precision%29))
  ;[1 1 1] Camera Inut
  (Pawn|Input|AddControllerYawInput (* AxisValue (Variables|CameraSetup|GetBaseTurnRate) (Utilities|Time|GetWorldDeltaSeconds))))

(event Input|AxisEvents|InputAxisLookUp
  (params (AxisValue :type Float%20%28single-precision%29))
  ;[1 1 1] Camera Inut
  (Pawn|Input|AddControllerPitchInput (* AxisValue (Variables|CameraSetup|GetBaseLookUpRate) (Utilities|Time|GetWorldDeltaSeconds))))

(fn ConstructionScript)

(fn SetMaxMinAddFunction
  (params (AxisValue :type Float%20%28single-precision%29))
  ;[0 0.3724 1] Limit Rotation angle
  (if (> AxisValue 0.0)
    ;;[0 0.3724 1] Right Rotation
    (Variables|Rotation|SetRotationMin 0.0)
    (Variables|Rotation|SetRotationMax 9e+01)
    (Variables|Rotation|SetRotationAdd -5.0)
    (elif (< AxisValue 0.0)
      ;;[0 0.3724 1] Left Rotation
      (Variables|Rotation|SetRotationMin -9e+01)
      (Variables|Rotation|SetRotationMax 0.0)
      (Variables|Rotation|SetRotationAdd 5.0)
      (elif (== AxisValue 0.0)
        _))))

(fn SetMaxMinAngle
  (params (InputAxis :type Float%20%28single-precision%29))
  (if (> InputAxis 0.0)
    (Variables|Default|SetMaxAngle 9e+01)
    (Variables|Default|SetMinAngle 0.0)
    (Variables|Default|SetToAdd 5.0)
    (elif (< InputAxis 0.0)
      (Variables|Default|SetMaxAngle 0.0)
      (Variables|Default|SetMinAngle -9e+01)
      (Variables|Default|SetToAdd -5.0))))
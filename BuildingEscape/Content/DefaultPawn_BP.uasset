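; Default pawn Blueprint that prototypes a physics-object grabber as a Blueprint equivalent of C++ code.
; Each tick it line-traces from the player's viewpoint along Reach for physics bodies, drawing the ray and printing the hit actor's name.
; BeginPlay reports whether physics handle and input components exist.
; Grab press calls the physics handle without passing it the traced component, and release only prints a message.
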(event EventBeginPlay
  ;[0.08635 1 0.04031] Begin Play_Equivalent of C++ in BP
  (Utilities|IsValid (Actor|GetComponentbyClass "/Script/Engine.PhysicsHandleComponent")
    (:Is%20Valid
      (Development|PrintString "Physics Handle Found" true true "(R=0.099934,G=1.000000,B=0.000000,A=1.000000)" 4.0))
    (:Is%20Not%20Valid
      (Development|PrintString "Physics Handle NOT Found" true true "(R=1.000000,G=0.000000,B=0.000000,A=1.000000)" 4.0)))
  (Utilities|IsValid (Actor|GetComponentbyClass "/Script/Engine.InputComponent")
    (:Is%20Valid
      (Development|PrintString "Input Component Found" true true "(R=0.099934,G=1.000000,B=0.000000,A=1.000000)" 4.0))
    (:Is%20Not%20Valid
      (Development|PrintString "Input Component NOT Found" true true "(R=1.000000,G=0.000000,B=0.000000,A=1.000000)" 4.0))))

(event EventTick
  (params (DeltaSeconds :type Float%20%28single-precision%29))
  ;[0.07005 0.2462 1] LineTrace_Equivalent of C++ in BP
  (CallFunction|DrawLineTrace))

(event Input|ActionEvents|InputActionGrab
  (params (Key :type Key%20Structure))
  (:Pressed
    (Development|PrintString "Grab Is Pressed!")
    (Class|PhysicsHandleComponent|GrabComponentatLocation (Variables|Default|GetPhysicsHandle) 0 "None" "0, 0, 0"))
  (:Released
    (Development|PrintString "Grab Is Released!")))

(fn ConstructionScript)

(fn DrawLineTrace
  (bind _returnvalue (Game|GetPlayerController 0))
  (bind (_outlocation _outrotation) (Actor|GetActorEyesViewPoint _returnvalue))
  ;[0 0.1091 1] DrawDebugLineTrace_BP Equivalent of C++
  (Variables|Default|SetPlayerViewPointLocation _outlocation)
  (Variables|Default|SetPlayerViewPointRotation _outrotation)
  (bind (_outhit _returnvalue_2) (Collision|LineTraceForObjects (Variables|Default|GetPlayerViewPointLocation) (+ (Variables|Default|GetPlayerViewPointLocation) (* (Math|Vector|GetForwardVector (Variables|Default|GetPlayerViewPointRotation)) (Variables|Default|GetReach))) (Utilities|Array|MakeArray "ObjectTypeQuery4") false 0 "ForOneFrame" true (Variables|Default|GetLineColor)))
  (if _returnvalue_2
    (Development|PrintString (Utilities|GetObjectName (.HitActor (Collision|BreakHitResult _outhit))) true true "(R=0.000000,G=0.660000,B=1.000000,A=1.000000)" 0.2)))
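; Ghost pawn that chases the Pacman player character.
; On BeginPlay it caches player 0's character as PacMan if that is a Pacman_BP.
; While FollowPacMan is set, Tick moves it toward PacMan by a fraction of the remaining offset scaled by Speed and delta time, so it slows as it closes in.
; The move is a direct SetActorLocation without sweep, so collision does not block it.
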(event EventBeginPlay
  ;[0 0.3724 1] Who is Pacman?
  (bind _aspacman_bp (Utilities|Casting|CastToPacman_BP (Game|GetPlayerCharacter 0)))
  (Variables|Default|SetPacMan _aspacman_bp))

(event EventTick
  (params (DeltaSeconds :type Float%20%28single-precision%29))
  ;[0 0.3724 1] Move Ghost
  (if (Variables|Setup|GetFollowPacMan?)
    (Transformation|SetActorLocation (+ (* (- (Transformation|GetActorLocation (Variables|Default|GetPacMan)) (Transformation|GetActorLocation)) (* DeltaSeconds (Variables|Setup|GetSpeed))) (Transformation|GetActorLocation)) false false)))

(fn ConstructionScript)
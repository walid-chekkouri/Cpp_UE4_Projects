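; Openable door actor that swings around its yaw axis when its OpenCloseDoor component fires open or close events.
; Open plays the DoorSwing timeline and close reverses it, adding the OpenAngle curve to the rotation stored at BeginPlay.
; An event track on the timeline times the door lock sound at the actor's location.
; BeginPlay also prints the result of a TestGround test call after a short delay.
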(event OnOpen(OpenCloseDoor)
  (bind _initialrotation (Variables|Default|GetInitialRotation))
  (bind _open_angle (Timeline|DoorSwing Play)
    (:Update
      (Transformation|SetActorRotation (Math|Rotator|MakeRotator (.roll _initialrotation) (.pitch _initialrotation) (+ _open_angle (.yaw _initialrotation)))))
    (:SoundTiming
      (Audio|PlaySoundatLocation "/Game/door-lock.door-lock" (Transformation|GetActorLocation) "0, 0, 0" 1.0 1.0 0.0 0 0 0))))

(event OnClose(OpenCloseDoor)
  (bind _initialrotation (Variables|Default|GetInitialRotation))
  (bind _open_angle (Timeline|DoorSwing Reverse)
    (:Update
      (Transformation|SetActorRotation (Math|Rotator|MakeRotator (.roll _initialrotation) (.pitch _initialrotation) (+ _open_angle (.yaw _initialrotation)))))
    (:SoundTiming
      (Audio|PlaySoundatLocation "/Game/door-lock.door-lock" (Transformation|GetActorLocation) "0, 0, 0" 1.0 1.0 0.0 0 0 0))))

(event EventBeginPlay
  (Variables|Default|SetInitialRotation (Transformation|GetActorRotation))
  (Utilities|FlowControl|Delay 2.0)
  (bind _returnvalue (Class|OpenDoor|TestGround (Variables|Default|GetOpenCloseDoor) "Sami" "The Rock" 21.0))
  (Development|PrintString _returnvalue true true "(R=1.000000,G=0.000000,B=0.789221,A=1.000000)" 6.0))

(fn ConstructionScript)